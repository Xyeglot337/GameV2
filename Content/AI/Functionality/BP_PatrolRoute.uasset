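; BP_PatrolRoute defines an AI patrol path from the points of its PatrolRout spline.
; It tracks a current point index and exposes that point's world position through GetSplinePointAsWorldPosition.
; IncrementPatrolRoute steps the index by Direction and reverses at the first and last points, so the route runs back and forth rather than looping.
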(event `IncrementPatrolRoute`
  (bind _output_get (set `self.PatrolIndex` (+ (`self.PatrolIndex`) (`self.Direction`))))
  (if (== _output_get (- (`SplineComponent.GetNumberOfSplinePoints` (`self.PatrolRout`)) 1))
    (set `self.Direction` -1)
    (elif (== (`self.PatrolIndex`) 0)
      (set `self.Direction` 1))))

(fn `GetSplinePointAsWorldPosition`
  (returns (Location :type "Vector Structure"))
  (return (`SplineComponent.GetLocationAtSplinePoint` (`self.PatrolRout`) (`self.PatrolIndex`) "World")))

(fn `UserConstructionScript`)