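; BP_Enemy_Base1 is a base enemy character Blueprint that provides player chasing, montage attacks and speed control for AI.
; Chasing uses AIMoveTo toward the player and, on success, waits briefly before calling ChasePlayer again.
; Attacks fire OnAttackEnd when the montage completes or is interrupted, and SetMovementSpeed maps movement states to walk speeds.
; Getters expose the patrol route plus animation, aim, hand-sway and IK state, with the left-hand socket getter left empty.
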(event `Chase_Player`
  (`|AIMoveTo` self (0.0 0.0 0.0) (`GameplayStatics.GetPlayerCharacter` 0) 150.0
    (:`OnSuccess`
      (`KismetSystemLibrary.Delay` 2.0)
      (`self.Chase_Player`))))

(event `Attack`
  (`|PlayMontage` (`self.Mesh`) "/Game/AI/Animations/AM_Enemy_Attack.AM_Enemy_Attack"
    (:`OnCompleted`
      _)
    (:`OnInterrupted`
      _))
  (`self.OnAttackEnd`))

(fn `GetPatrolRoute`
  (returns (PatrolRoute :type "/Game/AI/Functionality/BP_PatrolRoute Object Reference"))
  (return (`self.PatrolRoute`)))

(fn `IA_GetHandSwayFloats`
  (returns (SideMov :type "Float (double-precision)") (MouseX :type "Float (double-precision)") (MouseY :type "Float (double-precision)"))
  (return (`self.Side Mov`) (`self.Mouse X`) (`self.Mouse Y`)))

(fn `IF_GetAnimState`
  (returns (animState :type "/Game/ThirdPerson/Blueprints/Invetory/ItemData/AnimState Enum"))
  (return (`self.Anim State`)))

(fn `IF_GetIsAim`
  (returns (aim :type Boolean))
  (return (`self.Aiming`)))

(fn `IF_getLeftHandSocketTransform`
  (returns (leftHamdSocket :type "Transform Structure")))

(fn `IF_GetStopLeftHandIK`
  (returns (StopIK :type Boolean))
  (return (`self.StopLeftHandIk`)))

(fn `SetMovementSpeed`
  (params (Speed :type "/Game/AI/Functionality/Enums/E_MovementSpeed Enum" :default "NewEnumerator0"))
  (returns (SpeedValue :type "Float (double-precision)"))
  (bind _output_get (set `CharacterMovementComponent.MaxWalkSpeed` (select `/Game/AI/Functionality/Enums/E_MovementSpeed` Speed :`NewEnumerator1` 100.0 :`NewEnumerator2` 300.0 :`NewEnumerator3` 500.0 :!type "Float (single-precision)") (`self.CharacterMovement`)))
  (return _output_get))

(fn `UserConstructionScript`)