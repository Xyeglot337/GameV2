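; Base enemy Blueprint that provides an attack action and exposes animation state through interface functions.
; Attack plays an attack montage on the mesh and fires OnAttackEnd whether the montage completes or is interrupted.
; Interface getters return hand sway inputs, anim state, aiming and left-hand IK stop values, while the left-hand socket transform getter is an unwired stub.
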(event `self.ReceiveBeginPlay`)

(event `Attack`
  (`|PlayMontage` (`self.Mesh`) "/Game/AI/Animations/AM_Enemy_Attack.AM_Enemy_Attack"
    (:`OnCompleted`
      _)
    (:`OnInterrupted`
      _))
  (`self.OnAttackEnd`))

(fn `IA_GetHandSwayFloats`
  (returns (SideMov :type "Float (double-precision)") (MouseX :type "Float (double-precision)") (MouseY :type "Float (double-precision)"))
  (return (`self.Side Mov`) (`self.Mouse X`) (`self.Mouse Y`)))

(fn `IF_GetAnimState`
  (returns (animState :type "/Game/ThirdPerson/Blueprints/Invetory/ItemData/AnimState Enum"))
  (return (`self.Anim State`)))

(fn `IF_GetIsAim`
  (returns (aim :type Boolean))
  (return (`self.Aiming`)))

(fn `IF_getLeftHandSocketTransform`
  (returns (leftHamdSocket :type "Transform Structure")))

(fn `IF_GetStopLeftHandIK`
  (returns (StopIK :type Boolean))
  (return (`self.StopLeftHandIk`)))

(fn `UserConstructionScript`)