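; BP_OldInventory is a shop trigger actor that lets the player open the old shop's inventory with IA_Interact.
; Box overlap by the third-person character opens or closes a Gate, and both events call EnableInput.
; Interacting inside the box spawns the inventory through the character cached at BeginPlay and sets InOldShop, provided the shop is neither entered nor empty and F9DIsVisible is true.
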(event `self.ReceiveBeginPlay`
  (bind _asbp_third_person_character (cast `/Game/ThirdPerson/Blueprints/BP_ThirdPersonCharacter` (`GameplayStatics.GetPlayerCharacter` 0)))
  (set `self.As BP Third Person Character` _asbp_third_person_character))

(event `EnhancedInput|/Game/ThirdPerson/Input/Actions/IA_Interact`
  (params (ActionValue :type Boolean) (ElapsedSeconds :type "Float (double-precision)") (TriggeredSeconds :type "Float (double-precision)") (InputAction :type "InputAction Object Reference" :default "/Game/ThirdPerson/Input/Actions/IA_Interact.IA_Interact"))
  (bind _as_bp_third_person_character (`self.As BP Third Person Character`))
  (:`Triggered`
    (if (`/Game/ThirdPerson/Blueprints/BP_ThirdPersonCharacter.InOldShop?` _as_bp_third_person_character)
      _
      (elif (not (`/Game/ThirdPerson/Blueprints/BP_ThirdPersonCharacter.OldShopEmpty` _as_bp_third_person_character))
        (`/Engine/EditorBlueprintResources/StandardMacros.Gate` true :!label _label
          (:`Exit`
            (if (`/Game/ThirdPerson/Blueprints/BP_ThirdPersonCharacter.F9DIsVisible` _as_bp_third_person_character)
              (`KismetSystemLibrary.PrintString` "Buy")
              (`/Game/ThirdPerson/Blueprints/BP_ThirdPersonCharacter.SpawnOldInventory` _as_bp_third_person_character)
              (set `/Game/ThirdPerson/Blueprints/BP_ThirdPersonCharacter.InOldShop?` true _as_bp_third_person_character))))))))

(event `self.Box.OnComponentBeginOverlap`
  (params (OverlappedComponent :type "PrimitiveComponent Object Reference") (OtherActor :type "Actor Object Reference") (OtherComp :type "PrimitiveComponent Object Reference") (OtherBodyIndex :type Integer) (bFromSweep :type Boolean) (SweepResult :type "HitResult Structure (by ref)"))
  (cast `/Game/ThirdPerson/Blueprints/BP_ThirdPersonCharacter` OtherActor)
  (`self.EnableInput` (`GameplayStatics.GetPlayerController` 0))
  (goto _label :!via `Open`))

(event `self.Box.OnComponentEndOverlap`
  (params (OverlappedComponent :type "PrimitiveComponent Object Reference") (OtherActor :type "Actor Object Reference") (OtherComp :type "PrimitiveComponent Object Reference") (OtherBodyIndex :type Integer))
  (cast `/Game/ThirdPerson/Blueprints/BP_ThirdPersonCharacter` OtherActor)
  (`self.EnableInput` (`GameplayStatics.GetPlayerController` 0))
  (goto _label :!via `Close`))

(fn `UserConstructionScript`)